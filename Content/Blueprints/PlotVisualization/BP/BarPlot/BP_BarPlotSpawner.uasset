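; Bar plot spawner that generates BP_Bar actors from a data map or data table and rebuilds them when BP_TEST signals a data change.
; It extends a parent spawner's loop hooks, attaching each bar to a responsible actor and collecting its percentage, calculated unless already supplied.
; The end-of-loop hook sets bar heights, fills hidden hover widgets with name and value, then resets the totals.
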(event Custom|On%20Data%20Set%20Change
  ;[1 1 1] Calculate The Graph Again With New Input
  (Class|GenericSystem|RemoveGraphActors)
  (Class|GenericSystem|DataSetCreation)
  (CallFunction|DistributeActors))

(event EventBeginPlay
  (bind _returnvalue (Actor|GetActorOfClass "/Game/Blueprints/PlotVisualization/BP/BP_TEST.BP_TEST_C"))
  (EventDispatchers|BindEventtoSubscribetoDataChange _returnvalue (delegate Custom|On%20Data%20Set%20Change)))

(fn ConstructionScript)

(fn LoopCreator
  (|CallParentFunction)
  (if (Variables|Default|GetIsDataMapUsed)
    ;[1 1 1] Read the data length from data map
    (bind _keys (Utilities|Map|Keys (Variables|Default|GetDataMap)))
    (bind _output_get (Variables|Default|SetOut%20Row%20Names _keys))
    (Variables|Default|SetGenericIteratorLength (Utilities|Array|Length _output_get))
    (else
      ;[1 1 1] Read the data length and assign here
      (bind _outrownames (DataTable|GetDataTableRowNames (Variables|Default|GetData_Table)))
      (bind _output_get_2 (Variables|Default|SetOut%20Row%20Names _outrownames))
      (Variables|Default|SetGenericIteratorLength (Utilities|Array|Length _output_get_2))))
  ;[1 1 1] Assign the type of class
  (Variables|Default|SetGenericClass (Variables|Default|GetBar))
  (return (Variables|Default|GetGenericIteratorLength)))

(fn DistributeActors
  (|CallParentFunction))

(fn InLoopActorModifier
  (params (Actor :type Actor%20Object%20Reference))
  (|CallParentFunction Actor)
  (Utilities|FlowControl|Sequence
    (:then_0
      ;[1 0.6411 0] Add Each Bar Under Responsible Actor
      (Variables|Default|SetActor Actor)
      (Utilities|IsValid (Variables|Default|GetResponsibleActorInScene)
        (:Is%20Valid
          (Transformation|AttachActorToActor (Variables|Default|GetActor) (Variables|Default|GetResponsibleActorInScene) "None" "KeepRelative" "KeepRelative" "KeepWorld" true))))
    (:then_1
      ;[1 1 1] ADD BRANCHING 22.06.23
      (if (Variables|Default|GetIsDataMapUsed)
        (if (Variables|Default|GetIsAlreadyPercentage)
          ;;[1 1 1] Fill The Data Percentages Array From Data Map as Percentages
          (bind _values (Utilities|Map|Values (Variables|Default|GetDataMap)))
          (Utilities|Array|Add (Variables|Default|GetData%20Percentages) (Utilities|Array|Get(acopy) _values (Variables|Default|GetGenericIndex)))
          (else
            (bind _values_2 (Utilities|Map|Values (Variables|Default|GetDataMap)))
            (bind _returnvalue (Class|CalculatePercentage|CalculateDataPercentage (Variables|Default|GetCalculatePercentage) (Utilities|Array|Get(acopy) _values_2 (Variables|Default|GetGenericIndex))))
            (Utilities|Array|Add (Variables|Default|GetData%20Percentages) _returnvalue)))
        (elif (Variables|Default|GetIsAlreadyPercentage)
          ;;[0 0.1676 1] Fill Data Percentages Array With Percentages From Data Set
          (bind _returnvalue_2 (Utilities|GetDataTableRow (Variables|Default|GetData_Table) (Utilities|Array|Get(acopy) (Variables|Default|GetOut%20Row%20Names) (Variables|Default|GetGenericIndex)))
            (:then
              (Utilities|Array|Add (Variables|Default|GetData%20Percentages) (Utilities|Struct|BreakDummyDataStruct _returnvalue_2))))
          (else
            ;;[1 0 0.9496] Calculate Data Percentage and Fill The Array
            (bind _returnvalue_3 (Utilities|GetDataTableRow (Variables|Default|GetData_Table) (Utilities|Array|Get(acopy) (Variables|Default|GetOut%20Row%20Names) (Variables|Default|GetGenericIndex)))
              (:then
                (bind _returnvalue_4 (Class|CalculatePercentage|CalculateDataPercentage (Variables|Default|GetCalculatePercentage) (Utilities|Struct|BreakDummyDataStruct _returnvalue_3)))
                (Utilities|Array|Add (Variables|Default|GetData%20Percentages) _returnvalue_4)))))))))

(fn EndLoopActorModifier
  (|CallParentFunction)
  (Utilities|FlowControl|Sequence
    (:then_0
      ;[0 1 0.1776] Set Each Bar's Height
      (for (_array_element _array_index) (Actor|GetAttachedActors (Variables|Default|GetResponsibleActorInScene) true false)
        (bind _asbp_bar (Utilities|Casting|CastToBP_Bar _array_element)
          (:then
            (bind _output_get (Variables|/Game/Blueprints/PlotVisualization/BP/BarPlot/BP_Bar.BP_Bar_C|SetHeight%20of%20Bar _asbp_bar (Utilities|Array|Get(acopy) (Variables|Default|GetData%20Percentages) _array_index)))
            ;[1 1 1] Add UI Bars
            (Rendering|SetVisibility (Variables|/Game/Blueprints/PlotVisualization/BP/BarPlot/BP_Bar.BP_Bar_C|GetWidget _asbp_bar) false false)
            (bind _aswbp_on_hovering_data (Utilities|Casting|CastToWBP_OnHoveringData (UserInterface|GetWidget (Variables|/Game/Blueprints/PlotVisualization/BP/BarPlot/BP_Bar.BP_Bar_C|GetWidget _asbp_bar))))
            (Variables|/Game/Blueprints/Widgets/WBP_OnHoveringData.WBP_OnHoveringData_C|SetData%20%20Name _aswbp_on_hovering_data (Utilities|Text|ToText(Name) (Utilities|Array|Get(acopy) (Variables|Default|GetOut%20Row%20Names) _array_index)))
            (Variables|/Game/Blueprints/Widgets/WBP_OnHoveringData.WBP_OnHoveringData_C|SetData%20Value _aswbp_on_hovering_data (Utilities|Text|ToText(String) (Utilities|String|Append "%" (Utilities|String|ToString(Float) (* _output_get 1e+02))))))
          (:CastFailed
            (Development|PrintString "Cast Failed" true true "(R=1.000000,G=0.000000,B=0.005162,A=1.000000)" 55.0))))
      ;;[1 0 0] Reset Data Percentages for New Data Creation
      (Utilities|Array|Clear (Variables|Default|GetData%20Percentages)))
    (:then_1
      ;[1 0 0.01591] Reset Total Data Sum for New Data Creation
      (Variables|/Script/ProceduralSplines.CalculatePercentage|SetTotalDataSum (Variables|Default|GetCalculatePercentage) 0.0))))