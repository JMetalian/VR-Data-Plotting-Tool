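; BP_ParentAnchor is a plot visualization anchor that positions its HoritontalAxis component relative to the actors attached to it.
; Every Tick it loops over its directly attached actors and picks one by index: half the count when even, half plus one when odd.
; It moves the axis to that actor's world location, shifted along X by VerticalAxisPlacementOffset.
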(event EventBeginPlay)

(event Collision|EventActorBeginOverlap
  (params (OtherActor :type Actor%20Object%20Reference)))

(event EventTick
  (params (DeltaSeconds :type Float%20%28single-precision%29))
  (bind _vertical_axis_placement_offset (Variables|Default|GetVertical%20Axis%20Placement%20Offset))
  (bind _output_get (Variables|Default|SetOut%20Actors (Actor|GetAttachedActors true false)))
  (if (Utilities|Array|IsNotEmpty _output_get)
    (for (_array_element _array_index) (Variables|Default|GetOut%20Actors)
      (Variables|Default|SetArray%20Index _array_index)
      (Utilities|IsValid _array_element
        (:Is%20Valid
          (if (== (Math|Integer|%(Integer) (Utilities|Array|Length (Variables|Default|GetOut%20Actors)) 2) 0)
            (if (== (Variables|Default|GetArray%20Index) (/ (Utilities|Array|Length (Variables|Default|GetOut%20Actors)) 2))
              (Transformation|SetWorldLocation (Variables|Default|GetHoritontal%20Axis) (Math|Vector|MakeVector (+ (.x (Transformation|GetActorLocation (Utilities|Array|Get(acopy) (Variables|Default|GetOut%20Actors) (Variables|Default|GetArray%20Index)))) _vertical_axis_placement_offset) (.y (Transformation|GetActorLocation (Utilities|Array|Get(acopy) (Variables|Default|GetOut%20Actors) (Variables|Default|GetArray%20Index)))) (.z (Transformation|GetActorLocation (Utilities|Array|Get(acopy) (Variables|Default|GetOut%20Actors) (Variables|Default|GetArray%20Index))))) false false))
            (elif (== (+ (/ (Utilities|Array|Length (Variables|Default|GetOut%20Actors)) 2) 1) (Variables|Default|GetArray%20Index))
              (Transformation|SetWorldLocation (Variables|Default|GetHoritontal%20Axis) (Math|Vector|MakeVector (+ (.x (Transformation|GetActorLocation (Utilities|Array|Get(acopy) (Variables|Default|GetOut%20Actors) (Variables|Default|GetArray%20Index)))) _vertical_axis_placement_offset) (.y (Transformation|GetActorLocation (Utilities|Array|Get(acopy) (Variables|Default|GetOut%20Actors) (Variables|Default|GetArray%20Index)))) (.z (Transformation|GetActorLocation (Utilities|Array|Get(acopy) (Variables|Default|GetOut%20Actors) (Variables|Default|GetArray%20Index))))) false false))))))))

(fn ConstructionScript)