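; BP_TEST is a debug actor for testing plot visualization with different datasets through keyboard input.
; It enables player input on BeginPlay.
; Keys 1, 2 and 3 assign one of three data tables, the third for percentage data, to the referenced spawner's DataSet.
; Key 7 separately calls CallSubscribeToDataChange to test data creation, as the dataset keys only set the variable.
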(event EventBeginPlay
  ;[1 1 1] Test Player Input
  (Input|EnableInput (Game|GetPlayerController 0)))

(event Input|KeyboardEvents|1
  (params (Key :type Key%20Structure :default "None"))
  ;[1 1 1] Apply Different Datasets to Test
  (:Pressed
    (CallFunction|ApplyTestData1)))

(event Input|KeyboardEvents|2
  (params (Key :type Key%20Structure :default "None"))
  ;[1 1 1] Apply Different Datasets to Test
  (:Pressed
    (CallFunction|ApplyTestData2)))

(event Input|KeyboardEvents|7
  (params (Key :type Key%20Structure :default "None"))
  ;[1 1 1] Test Player Input
  ;;[1 1 1] Test Input For Data Creation
  (:Pressed
    (Default|CallSubscribetoDataChange)))

(event Input|KeyboardEvents|3
  (params (Key :type Key%20Structure :default "None"))
  ;[1 1 1] Apply Different Datasets to Test
  (:Pressed
    (CallFunction|ApplyTestDataPercentage)))

(fn ConstructionScript)

(fn ApplyTestData1
  (Variables|/Script/ProceduralSplines.GenericSystem|SetDataSet (Variables|Default|GetSpawner%20Reference) (Variables|Default|GetData%20Table%201)))

(fn ApplyTestData2
  (Variables|/Script/ProceduralSplines.GenericSystem|SetDataSet (Variables|Default|GetSpawner%20Reference) (Variables|Default|GetData%20Table%202)))

(fn ApplyTestDataPercentage
  (Variables|/Script/ProceduralSplines.GenericSystem|SetDataSet (Variables|Default|GetSpawner%20Reference) (Variables|Default|GetData%20Table%203)))