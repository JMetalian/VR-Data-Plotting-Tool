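; BP_GenericSpawner is a base spawner for plot visualization that lays out instances of GenericClass in a row.
; DistributeActors takes its count from LoopCreator and spawns actors at even Y intervals from ResponsibleActorInScene, at a fixed height.
; Each spawn passes to InLoopActorModifier, and EndLoopActorModifier runs after the loop.
; Both modifiers are empty and LoopCreator returns zero, so nothing spawns unless overridden.
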(fn ConstructionScript)

(fn LoopCreator
  (return 0))

(fn DistributeActors
  (bind _responsibleactorinscene (Variables|Default|GetResponsibleActorInScene))
  (bind _returnvalue (Transformation|GetActorLocation _responsibleactorinscene))
  (bind _iterator_value (CallFunction|LoopCreator))
  (for _index (range 0 (- _iterator_value 1))
    (bind _output_get (Variables|Default|SetGenericIndex _index))
    (bind _returnvalue_2 (Game|SpawnActorfromClass (Variables|Default|GetGenericClass) (Math|Transform|MakeTransform (Math|Vector|MakeVector (.x _returnvalue) (+ (* _output_get 150) (.y _returnvalue)) 25.0) "0, 0, 0" "1.000000,1.000000,1.000000") "Undefined" 0 0))
    (CallFunction|InLoopActorModifier _returnvalue_2))
  (CallFunction|EndLoopActorModifier))

(fn InLoopActorModifier
  (params (Actor :type Actor%20Object%20Reference)))

(fn EndLoopActorModifier)