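; BP_Cut is a Geometry Script generated mesh actor that builds a parametric cylinder with a rounded-rectangle window cut out of it.
; On rebuild, it appends the cylinder, then creates the window profile on a compute mesh, positioned from the cylinder dimensions and a height offset.
; The profile is extruded along Y into a cutter and boolean-subtracted from the cylinder.
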(event EventBeginPlay)

(event Collision|EventActorBeginOverlap
  (params (OtherActor :type Actor%20Object%20Reference)))

(event EventTick
  (params (DeltaSeconds :type Float%20%28single-precision%29)))

(event Events|EventOnRebuildGeneratedMesh
  (params (TargetMesh :type Dynamic%20Mesh%20Object%20Reference))
  (bind _cylinder_radius (Variables|Default|GetCylinder%20Radius))
  (bind _cylinderheight (Variables|Default|GetCylinderHeight))
  (bind _returnvalue (* _cylinderheight 2.0))
  (bind _returnvalue_2 (/ _returnvalue 2.0))
  (bind _returnvalue_3 (- _cylinder_radius _returnvalue_2))
  ;[1 1 1] Create a Cylinder
  (bind _output_get (Variables|Default|SetTarget%20Mesh TargetMesh))
  (GeometryScript|Primitives|AppendCylinder :TargetMesh _output_get :Radius (Variables|Default|GetCylinder%20Radius) :Height (Variables|Default|GetCylinderHeight) :RadialSteps (Variables|Default|GetRadial%20Steps) :HeightSteps (Variables|Default|GetHeight%20Steps) :Debug 0)
  ;[1 1 1] Set Window Cutting Parameters
  (bind _returnvalue_4 (DynamicMeshActor|AllocateComputeMesh))
  (Variables|Default|SetRadius%20Windows%20Offset _returnvalue_3)
  (bind _returnvalue_5 (Class|GeometryScriptLibraryMeshPrimitiveFunctions|AppendRoundRectangleXY :TargetMesh _returnvalue_4 :Transform (Math|Transform|MakeTransform (Math|Vector|MakeVector 0.0 _returnvalue_3 (+ (/ (Variables|Default|GetCylinderHeight) 2.0) (Variables|Default|GetWindow%20Height%20Offset) (/ (Variables|Default|GetCylinderHeight) 2.0))) (Variables|Default|GetTransform%20Rotation) "1.000000,1.000000,1.000000") :DimensionX (Variables|Default|GetWindow%20Width) :DimensionY (Variables|Default|GetWindow%20Height) :CornerRadius (Math|Float|Clamp(Float) (Variables|Default|GetWindow%20Corner%20Radius) 0.02 2.5e+02) :StepsRound (Variables|Default|GetWindow%20Step%20Round) :Debug 0))
  (bind _returnvalue_6 (Class|GeometryScriptLibraryMeshModelingFunctions|ApplyMeshExtrude _returnvalue_5 (Utilities|Struct|MakeGeometryScriptMeshExtrudeOptions 1.0 (Math|Vector|MakeVector 0.0 _returnvalue 0.0) 1.0 true) 0))
  ;[1 1 1] Apply Mesh on Target Mesh
  (Variables|Default|SetWindow%20Cutter%20Mesh _returnvalue_6)
  (bind _window_cutter_mesh (Variables|Default|GetWindow%20Cutter%20Mesh)
    (:then
      (GeometryScript|Booleans|ApplyMeshBoolean :TargetMesh (Variables|Default|GetTarget%20Mesh) :ToolMesh _window_cutter_mesh :Operation "Subtract" :Debug 0))
    (:else)))

(fn ConstructionScript)