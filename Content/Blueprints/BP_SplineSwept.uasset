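; Generated dynamic mesh actor that sweeps a Section spline's profile along a Path spline and appends a torus ring.
; Construction caches section points, an approximate radius and evenly spaced path samples.
; Mesh rebuild uses Geometry Script to sweep, repair normals and place the tangent-aligned ring, offset sideways by that radius.
; Tick applies a sine offset to a Path point indexed at point count minus -1, beyond the last valid index.
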(event EventBeginPlay
  (bind _path (Variables|Default|GetPath))
  (Variables|Default|SetInitial%20Location (Spline|GetLocationatSplinePoint _path (- (Spline|GetNumberOfSplinePoints _path) -1) "Local")))

(event Collision|EventActorBeginOverlap
  (params (OtherActor :type Actor%20Object%20Reference)))

(event EventTick
  (params (DeltaSeconds :type Float%20%28single-precision%29))
  (bind _path (Variables|Default|GetPath))
  (Spline|SetLocationatSplinePoint _path (- (Spline|GetNumberOfSplinePoints _path) -1) (+ (Variables|Default|GetInitial%20Location) (* (Math|Trig|Sin(Radians) (* (Utilities|Time|GetTimeSeconds) (Variables|Default|GetFrequency))) (Variables|Default|GetOffset))) "Local" true))

(event Events|EventOnRebuildGeneratedMesh
  (params (TargetMesh :type Dynamic%20Mesh%20Object%20Reference))
  (Variables|Default|SetTargetMesh TargetMesh)
  (bind _returnvalue (Class|GeometryScriptLibraryMeshPrimitiveFunctions|AppendSimpleSweptPolygon :TargetMesh (Variables|Default|GetTargetMesh) :PolygonVertices (Variables|Default|GetSectionPoints) :SweepPath (Variables|Default|GetPathPoints) :Debug 0))
  (Class|GeometryScriptLibraryMeshNormalsFunctions|AutoRepairNormals _returnvalue 0)
  (CallFunction|AddTorus))

(fn ConstructionScript
  (CallFunction|ReadSection)
  (CallFunction|ReadPath))

(fn ReadSection
  (bind _section (Variables|Default|GetSection))
  (Utilities|Array|Clear (Variables|Default|GetSectionPoints))
  (Variables|Default|SetSection%20Radius (Utilities|Operators|Divide (Spline|GetSplineLength _section) 2.0 (Math|Trig|GetPI)))
  (for _index (range 0 (- (Spline|GetNumberOfSplinePoints _section) 1))
    (Utilities|Array|Add (Variables|Default|GetSectionPoints) (Math|Vector2D|MakeVector2D (.x (Spline|GetLocationatSplinePoint _section _index "Local")) (.y (Spline|GetLocationatSplinePoint _section _index "Local"))))))

(fn ReadPath
  (Utilities|Array|Clear (Variables|Default|GetPathPoints))
  (for _index (range 0 (Variables|Default|GetNumber%20of%20SubSections))
    (Utilities|Array|Add (Variables|Default|GetPathPoints) (Spline|GetLocationatDistanceAlongSpline (Variables|Default|GetPath) (* (/ (Spline|GetSplineLength (Variables|Default|GetPath)) (Variables|Default|GetNumber%20of%20SubSections)) _index) "Local"))))

(fn AddTorus
  (bind _path (Variables|Default|GetPath))
  (bind _ring_location (Variables|Default|GetRing%20Location))
  (bind _returnvalue (Spline|GetTangentatDistanceAlongSpline _path _ring_location "World"))
  (bind _returnvalue_2 (Math|Rotator|MakeRotfromX _returnvalue))
  (bind _returnvalue_3 (Math|Vector|GetRightVector _returnvalue_2))
  (bind _returnvalue_4 (Math|Vector|Normalize _returnvalue_3))
  (Development|PrintString (Utilities|String|ToString(Vector) _returnvalue_4))
  (bind _returnvalue_5 (Class|GeometryScriptLibraryMeshPrimitiveFunctions|AppendTorus :TargetMesh (Variables|Default|GetTargetMesh) :Transform (Math|Transform|MakeTransform (+ (* _returnvalue_4 (Variables|Default|GetSection%20Radius) -1.0) (Spline|GetLocationatDistanceAlongSpline _path _ring_location "Local")) (Math|Rotator|MakeRotfromZ _returnvalue) "1.000000,1.000000,1.000000") :MajorRadius (Variables|Default|GetMajor%20Radius%20of%20Ring) :MinorRadius (Variables|Default|GetMinor%20Radius%20of%20Ring) :Debug 0))
  (Variables|Default|SetTorus%20Mesh _returnvalue_5))